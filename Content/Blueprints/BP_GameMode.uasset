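; BP_GameMode is a game mode that restores the player's saved location and rotation when play begins.
; On BeginPlay it checks the game instance's HasSavedGame flag, then loads the BP_SaveGame from the last used slot name.
; It applies the saved transform to the first player controller actor itself, rather than to its controlled pawn.
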(event EventBeginPlay
  (bind _returnvalue (Game|GetPlayerController 0))
  (bind _asbp_game_instance (Utilities|Casting|CastToBP_GameInstance (Game|GetGameInstance)))
  (if (Variables|/Game/Blueprints/BP_GameInstance.BP_GameInstance_C|GetHasSavedGame _asbp_game_instance)
    (bind _returnvalue_2 (SaveGame|LoadGamefromSlot (Variables|/Game/Blueprints/BP_GameInstance.BP_GameInstance_C|GetLastSaveSlotName _asbp_game_instance)))
    (bind _asbp_save_game (Utilities|Casting|CastToBP_SaveGame _returnvalue_2))
    (Transformation|SetActorLocation _returnvalue (Variables|/Game/Blueprints/SaveSystem/BP_SaveGame.BP_SaveGame_C|GetSavedPlayerLocation _asbp_save_game) false false)
    (Transformation|SetActorRotation _returnvalue (Variables|/Game/Blueprints/SaveSystem/BP_SaveGame.BP_SaveGame_C|GetSavedPlayerRotation _asbp_save_game))))

(fn ConstructionScript)