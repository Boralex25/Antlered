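; BP_Item is an interactable pickup actor that adds an item to the player's inventory.
; On BeginPlay it sets its mesh from its ItemData.
; Interact runs once, guarded by IsCollected: it hands ItemData to BP_GameInstance's inventory, destroys the actor and prints the picked-up item's name on screen in Russian.
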(event EventBeginPlay
  (Components|StaticMesh|SetStaticMesh (Variables|Default|GetItemMesh) (Variables|/Game/Blueprints/Data/DA_ItemData.DA_ItemData_C|GetMesh (Variables|Default|GetItemData))))

(event EventInteract
  (params (Instigator :type Actor%20Object%20Reference))
  (bind _itemdata (Variables|Default|GetItemData))
  (if (not (Variables|Default|GetIsCollected))
    (bind _asbp_game_instance (Utilities|Casting|CastToBP_GameInstance (Game|GetGameInstance)))
    (Default|AddItemtoInventory _asbp_game_instance _itemdata)
    (Variables|Default|SetIsCollected true)
    (Actor|DestroyActor)
    (Development|PrintString (Utilities|String|Append "Подобран: " (Utilities|String|ToString(Text) (Variables|/Game/Blueprints/Data/DA_ItemData.DA_ItemData_C|GetItemName _itemdata))) true true "(R=0.000000,G=0.000000,B=0.000000,A=1.000000)" 5.0)))

(fn ConstructionScript)