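; BP_Chaser is an AI enemy that kills the player on overlap; its event graph holds no movement logic.
; BeginPlay caches BP_Player and creates the death screen widget.
; On overlap it unregisters the player's perception stimulus, removes the default input mapping, plays the LS_TestDeath sequence and shows the death screen with cursor.
; LoadSavedGame teleports to the checkpoint through BP_GameInstance, then hides screen and cursor and restores input mapping.
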(event EventBeginPlay
  (bind _returnvalue (UserInterface|CreateWidget "/Game/UI/WBP_DeathScreen.WBP_DeathScreen_C"))
  (Variables|Default|SetDeathScreen _returnvalue)
  (bind _returnvalue_2 (Actor|GetActorOfClass "/Game/Blueprints/BP_Player.BP_Player_C"))
  (Variables|Default|SetPlayer _returnvalue_2))

(event EventLoadSavedGame
  (Development|PrintString "Hello" true true "(R=1.000000,G=0.791576,B=0.000000,A=1.000000)")
  (bind _asbp_game_instance (Utilities|Casting|CastToBP_GameInstance (Game|GetGameInstance)))
  (Default|TeleporttoCheckpoint _asbp_game_instance)
  (Variables|/Script/Engine.PlayerController|SetbShowMouseCursor (Game|GetPlayerController 0) false)
  (Widget|RemovefromParent (Variables|Default|GetDeathScreen))
  (Input|AddMappingContext (PlayerController|LocalPlayerSubsystems|GetEnhancedInputLocalPlayerSubsystem (Game|GetPlayerController (Variables|/Script/Engine.Pawn|GetPlayerState (Game|Player|GetPlayerPawn 0)))) "/Game/Input/IMC_Default.IMC_Default" 0 "(bIgnoreAllPressedKeysUntilRelease=True,bForceImmediately=False,bNotifyUserSettings=False)"))

(event Collision|EventActorBeginOverlap
  (params (OtherActor :type Actor%20Object%20Reference))
  (if (== OtherActor (Variables|Default|GetPlayer))
    (Class|AIPerceptionStimuliSourceComponent|UnregisterfromSense (Variables|/Game/Blueprints/BP_Player.BP_Player_C|GetAIPerceptionStimuliSource (Variables|Default|GetPlayer)) "/Script/AIModule.AISense")
    (Input|RemoveMappingContext (PlayerController|LocalPlayerSubsystems|GetEnhancedInputLocalPlayerSubsystem (Game|GetPlayerController (Variables|/Script/Engine.Pawn|GetPlayerState (Game|Player|GetPlayerPawn 0)))) "/Game/Input/IMC_Default.IMC_Default" "(bIgnoreAllPressedKeysUntilRelease=True,bForceImmediately=False,bNotifyUserSettings=False)")
    (bind _outactor (Sequencer|Player|CreateLevelSequencePlayer "/Game/Cutscenes/LS_TestDeath.LS_TestDeath"))
    (Sequencer|Player|Play (Variables|/Script/LevelSequence.LevelSequenceActor|GetSequencePlayer _outactor) :!class /Script/MovieScene.MovieSceneSequencePlayer)
    (UserInterface|Viewport|AddtoViewport (Variables|Default|GetDeathScreen) 0)
    (Variables|/Script/Engine.PlayerController|SetbShowMouseCursor (Game|GetPlayerController 0) true)))

(fn ConstructionScript)