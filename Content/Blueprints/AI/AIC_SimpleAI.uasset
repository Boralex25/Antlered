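; AIC_SimpleAI is an AI controller that drives a simple AI through the BT_SimpleAI behavior tree.
; On BeginPlay it runs the tree and stores the location of a BP_ReturnPoint actor found in the level as the ReturnLocation blackboard key.
; AI Perception updates set the TargetActor key to the sensed actor, or clear it when a stimulus is no longer successfully sensed.
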(event OnTargetPerceptionUpdated(AIPerception)
  (params (Actor :type Actor%20Object%20Reference) (Stimulus :type AI%20Stimulus%20Structure))
  (bind _returnvalue (AI|GetBlackboard 0))
  (if (.bsuccessfullysensed Stimulus)
    (AI|Components|Blackboard|SetValueasObject _returnvalue (Utilities|Name|MakeLiteralName "TargetActor") Actor)
    (else
      (AI|Components|Blackboard|SetValueasObject _returnvalue (Utilities|Name|MakeLiteralName "TargetActor") 0))))

(event EventBeginPlay
  (AI|RunBehaviorTree "/Game/Blueprints/AI/BT_SimpleAI.BT_SimpleAI")
  (bind _returnvalue (Actor|GetActorOfClass "/Game/Blueprints/AI/BP_ReturnPoint.BP_ReturnPoint_C"))
  (AI|Components|Blackboard|SetValueasVector (AI|GetBlackboard 0) (Utilities|Name|MakeLiteralName "ReturnLocation") (Transformation|GetActorLocation _returnvalue)))

(fn ConstructionScript)